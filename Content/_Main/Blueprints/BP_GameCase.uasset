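; BP_GameCase is a game case actor that can display a price tag and take a custom material.
; The price tag widget component starts hidden on BeginPlay.
; PutPriceTag casts the widget to W_PriceTag, sets its price text and shows it.
; SetGameCaseMaterial applies a given material instance to the second slot of the case mesh.
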(event `self.ReceiveBeginPlay`
  (`SceneComponent.SetVisibility` (`self.PriceWidget`) false false))

(event `PutPriceTag`
  (params (Price :type "Float (double-precision)"))
  (bind _asw_price_tag (cast `/Game/_Main/Widgets/W_PriceTag` (`WidgetComponent.GetUserWidgetObject` (`self.PriceWidget`))))
  (`/Game/_Main/Widgets/W_PriceTag.SetPriceText` _asw_price_tag Price)
  (`SceneComponent.SetVisibility` (`self.PriceWidget`) true false))

(event `SetGameCaseMaterial`
  (params (MatInstance :type "MaterialInstance Object Reference"))
  (`PrimitiveComponent.SetMaterial` (`self.SM_GameCase`) 1 MatInstance))

(fn `UserConstructionScript`)