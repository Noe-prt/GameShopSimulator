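; BP_Slot is an interactable slot that receives the game cases from the player's equipped BP_DeliveryBox for priced display.
; Hovering with a non-empty box toggles a preview material on its cube while the slot is not yet full.
; Interacting snaps each case onto the matching predefined place component and shows its market price tag.
; The slot then marks itself full, empties the box and hides the preview.
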(event `self.ReceiveBeginPlay`
  (set `self.GameCasesPlaces` (`|MakeArray` (`self.Box`) (`self.Box1`) (`self.Box2`) (`self.Box3`) (`self.Box4`) (`self.Box5`) (`self.Box6`) (`self.Box7`) (`self.Box8`) (`self.Box9`))))

(event `/Game/_Main/Blueprints/Interfaces/BPI_Hover.Hover/Unhover`
  (params (`Hover?` :type Boolean) (CharacterRef :type "/Game/_Main/Blueprints/Character/BP_FirstPersonCharacter Object Reference"))
  (bind _equippedactor (`/Game/_Main/Blueprints/Character/BP_FirstPersonCharacter.EquippedActor` CharacterRef)
    (:`then`
      (bind _asbp_delivery_box (cast `/Game/_Main/Blueprints/BP_DeliveryBox` _equippedactor))
      (if (`/Game/_Main/Blueprints/BP_DeliveryBox.Empty?` _asbp_delivery_box)
        _
        (elif (`self.SlotFull?`)
          _
          (elif `Hover?`
            (`PrimitiveComponent.SetMaterial` (`self.Cube`) 0 "/Game/_Main/Assets/Materials/MAT_Preview.MAT_Preview")
            (else
              (`PrimitiveComponent.SetMaterial` (`self.Cube`) 0 "/Game/_Main/Assets/Materials/M_Invisible.M_Invisible"))))))
    (:`else`)))

(event `/Game/_Main/Blueprints/Interfaces/BPI_Interact.Interact`
  (params (CharacterRef :type "/Game/_Main/Blueprints/Character/BP_FirstPersonCharacter Object Reference"))
  (bind _equippedactor (`/Game/_Main/Blueprints/Character/BP_FirstPersonCharacter.EquippedActor` CharacterRef)
    (:`then`
      (if (not (`self.SlotFull?`))
        (bind _asbp_delivery_box (cast `/Game/_Main/Blueprints/BP_DeliveryBox` _equippedactor))
        (if (not (`/Game/_Main/Blueprints/BP_DeliveryBox.Empty?` _asbp_delivery_box))
          (set `self.GameInfo` (`/Game/_Main/Blueprints/BP_DeliveryBox.GameInfo` _asbp_delivery_box))
          (for (_array_element _array_index) (`/Game/_Main/Blueprints/BP_DeliveryBox.GameCases` _asbp_delivery_box)
            (`self.K2_DetachFromActor` _array_element "KeepRelative" "KeepRelative" "KeepRelative")
            (`self.K2_AttachToComponent` _array_element (`|GetArrayItem` (`self.GameCasesPlaces`) _array_index) "None" "SnapToTarget" "SnapToTarget" "SnapToTarget" true)
            (`/Game/_Main/Blueprints/BP_GameCase.ShowPriceTag` _array_element (`.MarketPrice_16_0456552F40B30F3DB01BBDB84C9DBAE9` (break `/Game/_Main/Blueprints/Structures/S_Game` (`self.GameInfo`)))))
          (set `self.SlotFull?` true)
          (`/Game/_Main/Blueprints/BP_DeliveryBox.ClearBox` _asbp_delivery_box)
          (`PrimitiveComponent.SetMaterial` (`self.Cube`) 0 "/Game/_Main/Assets/Materials/M_Invisible.M_Invisible"))))
    (:`else`)))

(fn `UserConstructionScript`)