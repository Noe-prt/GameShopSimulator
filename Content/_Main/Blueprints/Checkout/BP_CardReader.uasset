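; BP_CardReader is the checkout card terminal the player operates to charge a client who pays by card.
; Receiving a card shows the card mesh, stores price and client, and enables hover outline and interaction.
; Interacting blends the view to the reader, locks movement, switches to UI-only input and passes the price to its W_CardReader widget.
; Completion adds cash through the game mode and finishes the client's purchase; completion or cancellation resets the reader and restores control.
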(event `/Game/_Main/Blueprints/Interfaces/BPI_Hover.Hover/Unhover`
  (params (`Hover?` :type Boolean) (CharacterRef :type "/Game/_Main/Blueprints/Character/BP_FirstPersonCharacter Object Reference"))
  (bind _mainwidgetref (`/Game/_Main/Blueprints/Character/BP_FirstPersonCharacter.MainWidgetRef` CharacterRef))
  (if (`self.HasCardInserted?`)
    (if `Hover?`
      (`MeshComponent.SetOverlayMaterial` (`self.Cylinder`) "/Game/_Main/Assets/Materials/MI_Hover_Outline.MI_Hover_Outline")
      (`MeshComponent.SetOverlayMaterial` (`self.Cube`) "/Game/_Main/Assets/Materials/MI_Hover_Outline.MI_Hover_Outline")
      (`MeshComponent.SetOverlayMaterial` (`self.Cylinder1`) "/Game/_Main/Assets/Materials/MI_Hover_Outline.MI_Hover_Outline")
      (`/Game/_Main/Widgets/W_MainWidget.SpawnInteractBox` _mainwidgetref)
      (else
        (`MeshComponent.SetOverlayMaterial` (`self.Cylinder1`) null)
        (`MeshComponent.SetOverlayMaterial` (`self.Cube`) null)
        (`MeshComponent.SetOverlayMaterial` (`self.Cylinder`) null)
        (`/Game/_Main/Widgets/W_MainWidget.DespawnInteractBox` _mainwidgetref)))))

(event `ReceiveCreditCard`
  (params (Price :type "Float (double-precision)") (ClientRef :type "/Game/_Main/Blueprints/Client/BP_Client Object Reference"))
  (`SceneComponent.SetVisibility` (`self.CardMesh`) true false)
  (set `self.HasCardInserted?` true)
  (set `self.Price` Price)
  (set `self.ClientRef` ClientRef))

(event `/Game/_Main/Blueprints/Interfaces/BPI_Interact.Interact`
  (params (CharacterRef :type "/Game/_Main/Blueprints/Character/BP_FirstPersonCharacter Object Reference"))
  (bind _returnvalue (`GameplayStatics.GetPlayerController` 0))
  (set `self.Character Ref` CharacterRef)
  (if (`self.HasCardInserted?`)
    (`/Game/_Main/Widgets/W_MainWidget.DespawnInteractBox` (`/Game/_Main/Blueprints/Character/BP_FirstPersonCharacter.MainWidgetRef` CharacterRef))
    (`MeshComponent.SetOverlayMaterial` (`self.Cylinder1`) null)
    (`MeshComponent.SetOverlayMaterial` (`self.Cube`) null)
    (`MeshComponent.SetOverlayMaterial` (`self.Cylinder`) null)
    (`PlayerController.SetViewTargetWithBlend` _returnvalue self 0.5 "VTBlend_Linear" 0.0 false)
    (set `PlayerController.bShowMouseCursor` true _returnvalue)
    (`WidgetBlueprintLibrary.SetInputMode_UIOnlyEx` _returnvalue null)
    (`CharacterMovementComponent.DisableMovement` (`Character.CharacterMovement` CharacterRef))
    (bind _asw_card_reader (cast `/Game/_Main/Widgets/W_CardReader` (`WidgetComponent.GetUserWidgetObject` (`self.CardReaderWidget`))))
    (`/Game/_Main/Widgets/W_CardReader.SetTotalPrice` _asw_card_reader (`self.Price`) self)))

(event `OnPurchasedCompleted`
  (bind _returnvalue (`GameplayStatics.GetPlayerController` 0))
  (bind _gamemoderef (message `/Game/_Main/Blueprints/Interfaces/BPI_GameMode.GetGameModeRef` (`GameplayStatics.GetGameMode`)))
  (`/Game/_Main/Blueprints/GM_GameShopSimulator.AddCash` _gamemoderef (`self.Price`))
  (set `self.Price` 0.0)
  (`PlayerController.SetViewTargetWithBlend` _returnvalue (`self.Character Ref`) 0.5 "VTBlend_Linear" 0.0 false)
  (set `PlayerController.bShowMouseCursor` false _returnvalue)
  (`WidgetBlueprintLibrary.SetInputMode_GameOnly` _returnvalue)
  (`CharacterMovementComponent.SetMovementMode` (`Character.CharacterMovement` (`self.Character Ref`)) "MOVE_Walking" 0)
  (set `self.HasCardInserted?` false)
  (`SceneComponent.SetVisibility` (`self.CardMesh`) false false)
  (`/Game/_Main/Blueprints/Client/BP_Client.FinishPurchase` (`self.ClientRef`))
  (set `self.ClientRef` null))

(event `OnPurchaseCanceled`
  (bind _returnvalue (`GameplayStatics.GetPlayerController` 0))
  (set `self.Price` 0.0)
  (set `PlayerController.bShowMouseCursor` false _returnvalue)
  (`WidgetBlueprintLibrary.SetInputMode_GameOnly` _returnvalue)
  (`/Engine/EditorBlueprintResources/StandardMacros.IsValid` (`self.Character Ref`)
    (:`Is Valid`
      (`PlayerController.SetViewTargetWithBlend` _returnvalue (`self.Character Ref`) 0.5 "VTBlend_Linear" 0.0 false)
      (`CharacterMovementComponent.SetMovementMode` (`Character.CharacterMovement` (`self.Character Ref`)) "MOVE_Walking" 0))
    (:`Is Not Valid`
      _))
  (set `self.HasCardInserted?` false)
  (`SceneComponent.SetVisibility` (`self.CardMesh`) false false)
  (set `self.ClientRef` null)
  (bind _asw_card_reader (cast `/Game/_Main/Widgets/W_CardReader` (`WidgetComponent.GetUserWidgetObject` (`self.CardReaderWidget`))))
  (`/Game/_Main/Widgets/W_CardReader.ClearDisplay` _asw_card_reader))

(fn `UserConstructionScript`)