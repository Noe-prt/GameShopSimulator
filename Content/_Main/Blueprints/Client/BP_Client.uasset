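; Customer AI for a game store that shops, pays or leaves, and reports the outcome to the game mode.
; ClientMoveToShelf starts an AIMoveTo chain with retries: shelf, popularity-weighted game choice, matching slot, then a probabilistic price check.
; Buyers carry the case to checkout, feed the display and card reader, and cancel if not served before a timer expires.
; Every outcome ends in ClientExit, showing speech text before walking out and despawning.
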(event `self.ReceiveBeginPlay`
  (`SkeletalMeshComponent.SetSkeletalMeshAsset` (`self.Mesh`) (`KismetArrayLibrary.Array_Random` (`self.ClientsMeshes`)))
  (bind _gamemoderef (message `/Game/_Main/Blueprints/Interfaces/BPI_GameMode.GetGameModeRef` (`GameplayStatics.GetGameMode`)))
  (set `self.Game Mode Ref` _gamemoderef)
  (bind _asw_client_text (cast `/Game/_Main/Widgets/W_ClientText` (`WidgetComponent.GetUserWidgetObject` (`self.Widget`))))
  (set `self.ClientWidgetRef` _asw_client_text))

(event `ClientMoveToShelf`
  (bind _targetslot (`self.TargetSlot`))
  (bind _gameinfo (`/Game/_Main/Blueprints/GameCase/BP_Slot.GameInfo` _targetslot))
  (bind _price (`/Game/_Main/Blueprints/GameCase/BP_Slot.Price` _targetslot))
  (bind ((`Name_2_7F26A8CE4D0FC23CA2007DB6CFD7ED73` _name) (`MarketPrice_16_0456552F40B30F3DB01BBDB84C9DBAE9` _marketprice)) (break `/Game/_Main/Blueprints/Structures/S_Game` _gameinfo))
  (bind _returnvalue (`GameplayStatics.GetActorOfClass` "/Game/_Main/Blueprints/Client/BP_AIShelfPoint.BP_AIShelfPoint_C"))
  (`|AIMoveTo` self (0.0 0.0 0.0) _returnvalue 50.0 :!label _label
    (:`OnSuccess`
      (`KismetSystemLibrary.Delay` 1.0)
      (bind (_found_ _targetgame) (`self.ChooseTargetGameByPopularity` (`/Game/_Main/Blueprints/GM_GameShopSimulator.Games` (`self.Game Mode Ref`))))
      (if _found_
        (bind (_found__2 _targetslot_2) (`self.GetSlotWithTargetGame` _targetgame))
        (if _found__2
          (set `self.TargetSlot` _targetslot_2)
          (`|AIMoveTo` self (`self.K2_GetActorLocation` (`self.TargetSlot`)) null 50.0 :!label _label_2
            (:`OnSuccess`
              (if (> _price 0.0)
                (bind _shouldbuy_ (`self.ShouldClientBuy` _gameinfo _price))
                (if _shouldbuy_
                  (`self.ClientTryTakeGame`)
                  (else
                    (`self.ClientExit` (make `ClientReport` false "TooExpensive" _marketprice _price) (`|FormatText` "\"{GameName} is way too expensive here… I'm leaving.\"" _name))))
                (else
                  (`self.ClientExit` (make `ClientReport` false "NoPrice") (`|FormatText` "{GameName} doesn’t even have a price tag…" (`.Name_2_7F26A8CE4D0FC23CA2007DB6CFD7ED73` (break `/Game/_Main/Blueprints/Structures/S_Game` _gameinfo)))))))
            (:`OnFail`
              (`KismetSystemLibrary.Delay` 1.0)
              (goto _label_2)))
          (else
            (`self.ClientExit` (make `ClientReport` false "NotFound") (`|FormatText` "\"I looked for {GameName}, but it's not here.\"" (`.Name_2_7F26A8CE4D0FC23CA2007DB6CFD7ED73` (break `/Game/_Main/Blueprints/Structures/S_Game` _targetgame))))))))
    (:`OnFail`
      (`KismetSystemLibrary.Delay` 1.0)
      (goto _label))))

(event `ClientExit`
  (params (ClientReport :type "ClientReport Structure") (Text :type Text))
  (`/Game/_Main/Blueprints/GM_GameShopSimulator.RegisterClientReport` (`self.Game Mode Ref`) ClientReport)
  (`KismetSystemLibrary.Delay` 1.0)
  (`/Game/_Main/Widgets/W_ClientText.ShowClientText` (`self.ClientWidgetRef`) Text 3.0)
  (bind _returnvalue (`GameplayStatics.GetActorOfClass` "/Game/_Main/Blueprints/Client/BP_AIExitPoint.BP_AIExitPoint_C"))
  (`|AIMoveTo` self (0.0 0.0 0.0) _returnvalue :!label _label_3
    (:`OnSuccess`
      (bind _targetgamecase (`self.TargetGameCase`)
        (:`then`
          (`self.K2_DestroyActor` _targetgamecase))
        (:`else`
          _))
      (`self.K2_DestroyActor`))
    (:`OnFail`
      (`KismetSystemLibrary.Delay` 1.0)
      (goto _label_3))))

(event `ClientTryTakeGame`
  (bind _output (`|GetArrayItem` (`/Game/_Main/Blueprints/GameCase/BP_Slot.GameCases` (`self.TargetSlot`))))
  (`KismetSystemLibrary.Delay` 1.0)
  (`/Engine/EditorBlueprintResources/StandardMacros.IsValid` _output
    (:`Is Valid`
      (bind _output_get (set `self.TargetGameCase` _output))
      (`self.K2_DetachFromActor` _output_get "KeepRelative" "KeepRelative" "KeepRelative")
      (`self.K2_AttachToComponent` (`self.TargetGameCase`) (`self.Mesh`) "S_GameCase" "SnapToTarget" "SnapToTarget" "SnapToTarget" true)
      (`/Game/_Main/Blueprints/GameCase/BP_Slot.UpdateSlot` (`self.TargetSlot`))
      (bind _returnvalue (`GameplayStatics.GetActorOfClass` "/Game/_Main/Blueprints/Client/BP_CheckoutPoint.BP_CheckoutPoint_C"))
      (`|AIMoveTo` self (0.0 0.0 0.0) _returnvalue :!label _label_4
        (:`OnSuccess`
          (bind _targetgamecase (`self.TargetGameCase`)
            (:`then`
              (`self.K2_DetachFromActor` _targetgamecase "KeepRelative" "KeepRelative" "KeepRelative")
              (bind _returnvalue_2 (`GameplayStatics.GetActorOfClass` "/Game/_Main/Blueprints/Client/BP_ScannerPoint.BP_ScannerPoint_C"))
              (`self.K2_SetActorTransform` _targetgamecase (`self.GetTransform` _returnvalue_2) false false)
              (bind _returnvalue_3 (`GameplayStatics.GetActorOfClass` "/Game/_Main/Blueprints/Checkout/BP_CheckoutDisplay.BP_CheckoutDisplay_C"))
              (bind _output_get_2 (set `self.CheckoutDisplayRef` _returnvalue_3))
              (bind _price (`/Game/_Main/Blueprints/GameCase/BP_GameCase.Price` _targetgamecase))
              (`/Game/_Main/Blueprints/Checkout/BP_CheckoutDisplay.AddItemToCheckoutWidget` _output_get_2 (`/Game/_Main/Blueprints/GameCase/BP_GameCase.GameInfo` _targetgamecase) _price)
              (bind _returnvalue_4 (`GameplayStatics.GetActorOfClass` "/Game/_Main/Blueprints/Checkout/BP_CardReader.BP_CardReader_C"))
              (set `self.CardReaderRef` _returnvalue_4)
              (`KismetSystemLibrary.Delay` 1.0)
              (`/Game/_Main/Blueprints/Checkout/BP_CardReader.ReceiveCreditCard` (`self.CardReaderRef`) _price self)
              (`KismetSystemLibrary.K2_SetTimerDelegate` (delegate `OnWaitTimeEnd`) (`self.WaitTime`)))
            (:`else`)))
        (:`OnFail`
          (`KismetSystemLibrary.Delay` 1.0)
          (goto _label_4))))
    (:`Is Not Valid`
      (`self.ClientExit` (make `ClientReport` false "NotFound") (`|FormatText` "\"I looked for {GameName}, but it's not here.\"" (`.Name_2_7F26A8CE4D0FC23CA2007DB6CFD7ED73` (break `/Game/_Main/Blueprints/Structures/S_Game` (`/Game/_Main/Blueprints/GameCase/BP_Slot.GameInfo` (`self.TargetSlot`)))))))))

(event `OnWaitTimeEnd`
  (if (not (`self.PurchaseComplete?`))
    (`self.CancelPurchase`)))

(event `FinishPurchase`
  (bind _targetgamecase (`self.TargetGameCase`))
  (bind ((`Name_2_7F26A8CE4D0FC23CA2007DB6CFD7ED73` _name) (`MarketPrice_16_0456552F40B30F3DB01BBDB84C9DBAE9` _marketprice)) (break `/Game/_Main/Blueprints/Structures/S_Game` (`/Game/_Main/Blueprints/GameCase/BP_GameCase.GameInfo` _targetgamecase)))
  (`/Game/_Main/Blueprints/Checkout/BP_CheckoutDisplay.ClearCheckOutDisplay` (`self.CheckoutDisplayRef`))
  (`self.K2_AttachToComponent` (`self.TargetGameCase`) (`self.Mesh`) "S_GameCase" "SnapToTarget" "SnapToTarget" "SnapToTarget" true)
  (set `self.PurchaseComplete?` true)
  (`self.ClientExit` (make `ClientReport` true "None" _marketprice (`/Game/_Main/Blueprints/GameCase/BP_GameCase.Price` _targetgamecase)) (`|FormatText` "\"Happy I found {GameName}! I'll come back.\"" _name)))

(event `CancelPurchase`
  (`/Game/_Main/Blueprints/Checkout/BP_CheckoutDisplay.ClearCheckOutDisplay` (`self.CheckoutDisplayRef`))
  (`self.K2_DestroyActor` (`self.TargetGameCase`))
  (`/Game/_Main/Blueprints/Checkout/BP_CardReader.OnPurchaseCanceled` (`self.CardReaderRef`))
  (`self.ClientExit` (make `ClientReport` false "NoCashier") "\"Nobody at checkout… I'm leaving.\""))

(fn `ChooseTargetGameByPopularity`
  (params (Games :type "Array of /Game/_Main/Blueprints/Structures/S_Game Structure"))
  (returns (`Found?` :type Boolean) (TargetGame :type "/Game/_Main/Blueprints/Structures/S_Game Structure"))
  (locals (totalWeight :type "Float (double-precision)") (result :type "Float (double-precision)") (accum :type "Float (double-precision)") (LocalGames :type "Array of /Game/_Main/Blueprints/Structures/S_Game Structure"))
  (bind _localgames (`local.LocalGames`))
  (bind _output_get (set `local.LocalGames` Games))
  (for _array_element _output_get
    (bind (_name _texture _material _marketprice _unitprice _unitsperbox _popularity) (break `/Game/_Main/Blueprints/Structures/S_Game` _array_element))
    (if (> _popularity 0.0)
      (set `local.totalWeight` (+ (`local.totalWeight`) _popularity))))
  (if (<= (`local.totalWeight`) 0.0)
    (return false)
    (else
      (set `local.result` (`KismetMathLibrary.RandomFloatInRange` 0.0 (`local.totalWeight`)))
      (for _array_element_2 (`local.LocalGames`)
        (set `local.accum` (+ (`local.accum`) (`.Popularity_23_A4FD008042D9E5138AC2E5B51CEC558E` (break `/Game/_Main/Blueprints/Structures/S_Game` _array_element_2))))
        (if (<= (`local.result`) (`local.accum`))
          (return true _array_element_2)))
      (return true (`|GetArrayItem` _localgames (`KismetArrayLibrary.Array_LastIndex` _localgames))))))

(fn `GetSlotWithTargetGame`
  (params (TargetGame :type "/Game/_Main/Blueprints/Structures/S_Game Structure"))
  (returns (`Found?` :type Boolean) (TargetSlot :type "/Game/_Main/Blueprints/GameCase/BP_Slot Object Reference"))
  (locals (SlotsWithTargetGames :type "Array of /Game/_Main/Blueprints/GameCase/BP_Slot Object Reference"))
  (bind _outactors (`GameplayStatics.GetAllActorsOfClass` "/Game/_Main/Blueprints/GameCase/BP_Slot.BP_Slot_C"))
  (for _array_element _outactors
    (if (`/Game/_Main/Blueprints/GameCase/BP_Slot.ContainGames` _array_element)
      (if (`KismetTextLibrary.EqualEqual_TextText` (`.Name_2_7F26A8CE4D0FC23CA2007DB6CFD7ED73` (break `/Game/_Main/Blueprints/Structures/S_Game` (`/Game/_Main/Blueprints/GameCase/BP_Slot.GameInfo` _array_element))) (`.Name_2_7F26A8CE4D0FC23CA2007DB6CFD7ED73` (break `/Game/_Main/Blueprints/Structures/S_Game` TargetGame)))
        (`KismetArrayLibrary.Array_Add` (`local.SlotsWithTargetGames`) _array_element))))
  (if (`KismetArrayLibrary.Array_IsEmpty` (`local.SlotsWithTargetGames`))
    (return false null)
    (else
      (return true (`KismetArrayLibrary.Array_Random` (`local.SlotsWithTargetGames`))))))

(fn `ShouldClientBuy`
  (params (GameInfo :type "/Game/_Main/Blueprints/Structures/S_Game Structure") (Price :type "Float (double-precision)"))
  (returns (`ShouldBuy?` :type Boolean))
  (locals (PurchaseProbability :type "Float (double-precision)") (random :type "Float (double-precision)"))
  (bind ((`MarketPrice_16_0456552F40B30F3DB01BBDB84C9DBAE9` _marketprice) (`Popularity_23_A4FD008042D9E5138AC2E5B51CEC558E` _popularity)) (break `/Game/_Main/Blueprints/Structures/S_Game` GameInfo))
  (bind _output_get (set `local.PurchaseProbability` (`ClientSimLibrary.ComputePurchaseProbability` _marketprice Price _popularity (`self.BasePriceSensitivity`) (`self.PerceptionThreshold`))))
  (`KismetSystemLibrary.PrintString` (`KismetStringLibrary.Conv_DoubleToString` _output_get))
  (set `local.random` (`KismetMathLibrary.RandomFloatInRange` 0.0 1.0))
  (if (<= (`local.random`) (`local.PurchaseProbability`))
    (return true)
    (else
      (return false))))

(fn `UserConstructionScript`)