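; BP_Computer is an interactable computer that toggles the player between walking and a computer-use view.
; Interacting makes the character drop, disables movement, shows the cursor with Game and UI input and blends the camera to the computer; interacting again reverses the mode and view.
; Hover events toggle an outline overlay material and the interact prompt on the character's main widget, which computer mode hides.
; GetComputerRef returns the actor itself.
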(event `/Game/_Main/Blueprints/Interfaces/BPI_Interact.Interact`
  (params (CharacterRef :type "/Game/_Main/Blueprints/Character/BP_FirstPersonCharacter Object Reference"))
  (bind _returnvalue (`GameplayStatics.GetPlayerController` 0))
  (bind _returnvalue_2 (`GameplayStatics.GetPlayerController` 0))
  (set `self.Character Ref` CharacterRef)
  (if (not (`self.ComputerMode?`))
    (`/Game/_Main/Blueprints/Character/BP_FirstPersonCharacter.Drop` (`self.Character Ref`))
    (set `PlayerController.bShowMouseCursor` true _returnvalue)
    (`WidgetBlueprintLibrary.SetInputMode_GameAndUIEx` _returnvalue null)
    (`CharacterMovementComponent.DisableMovement` (`Character.CharacterMovement` (`self.Character Ref`)))
    (`PlayerController.SetViewTargetWithBlend` _returnvalue self 0.3 "VTBlend_Linear" 0.0 false)
    (set `self.ComputerMode?` true)
    (`MeshComponent.SetOverlayMaterial` (`self.StaticMesh`) null)
    (`/Game/_Main/Widgets/W_MainWidget.DespawnInteractBox` (`/Game/_Main/Blueprints/Character/BP_FirstPersonCharacter.MainWidgetRef` (`self.Character Ref`)))
    (else
      (set `PlayerController.bShowMouseCursor` false _returnvalue_2)
      (`WidgetBlueprintLibrary.SetInputMode_GameOnly` _returnvalue_2)
      (`CharacterMovementComponent.SetMovementMode` (`Character.CharacterMovement` (`self.Character Ref`)) "MOVE_Walking" 0)
      (`PlayerController.SetViewTargetWithBlend` _returnvalue_2 (`self.Character Ref`) 0.3 "VTBlend_Linear" 0.0 false)
      (set `self.ComputerMode?` false)
      (`MeshComponent.SetOverlayMaterial` (`self.StaticMesh`) "/Game/_Main/Assets/Materials/MI_Hover_Outline.MI_Hover_Outline")
      (`/Game/_Main/Widgets/W_MainWidget.SpawnInteractBox` (`/Game/_Main/Blueprints/Character/BP_FirstPersonCharacter.MainWidgetRef` (`self.Character Ref`))))))

(event `/Game/_Main/Blueprints/Interfaces/BPI_Hover.Hover/Unhover`
  (params (`Hover?` :type Boolean) (CharacterRef :type "/Game/_Main/Blueprints/Character/BP_FirstPersonCharacter Object Reference"))
  (bind _mainwidgetref (`/Game/_Main/Blueprints/Character/BP_FirstPersonCharacter.MainWidgetRef` CharacterRef))
  (if `Hover?`
    (`MeshComponent.SetOverlayMaterial` (`self.StaticMesh`) "/Game/_Main/Assets/Materials/MI_Hover_Outline.MI_Hover_Outline")
    (`/Game/_Main/Widgets/W_MainWidget.SpawnInteractBox` _mainwidgetref)
    (else
      (`MeshComponent.SetOverlayMaterial` (`self.StaticMesh`) null)
      (`/Game/_Main/Widgets/W_MainWidget.DespawnInteractBox` _mainwidgetref))))

(fn `GetComputerRef`
  (returns (ComputerRef :type "/Game/_Main/Blueprints/Computer/BP_Computer Object Reference"))
  (return self))

(fn `UserConstructionScript`)