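; BP_DeliveryBox is an interactable, physics-simulated delivery box that holds game cases and can be carried by the character.
; AddGamesCasesToBox stores the GameInfo, waits briefly, then spawns one BP_GameCase per unit at preset slot transforms, attached to the mesh.
; Hovering toggles an outline overlay and interact widget.
; Interacting drops the held item, disables physics and collision, and attaches the box to the character; ClearBox empties the case list and flags Empty.
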(event `self.ReceiveBeginPlay`
  (set `self.GameCasesPlaces` (`|MakeArray` (`self.GameSpawn1`) (`self.GameSpawn2`) (`self.GameSpawn3`) (`self.GameSpawn4`) (`self.GameSpawn5`) (`self.GameSpawn6`) (`self.GameSpawn7`) (`self.GameSpawn8`) (`self.GameSpawn9`) (`self.GameSpawn10`) (`self.GameSpawn11`) (`self.GameSpawn12`) (`self.GameSpawn13`) (`self.GameSpawn14`)))
  (`PrimitiveComponent.SetSimulatePhysics` (`self.SM_Equippable`) true))

(event `/Game/_Main/Blueprints/Interfaces/BPI_Hover.Hover/Unhover`
  (params (`Hover?` :type Boolean) (CharacterRef :type "/Game/_Main/Blueprints/Character/BP_FirstPersonCharacter Object Reference"))
  (bind _mainwidgetref (`/Game/_Main/Blueprints/Character/BP_FirstPersonCharacter.MainWidgetRef` CharacterRef))
  (if `Hover?`
    (`MeshComponent.SetOverlayMaterial` (`self.SM_Equippable`) "/Game/_Main/Assets/Materials/MI_Hover_Outline.MI_Hover_Outline")
    (`/Game/_Main/Widgets/W_MainWidget.SpawnInteractBox` _mainwidgetref)
    (else
      (`MeshComponent.SetOverlayMaterial` (`self.SM_Equippable`) null)
      (`/Game/_Main/Widgets/W_MainWidget.DespawnInteractBox` _mainwidgetref))))

(event `AddGamesCasesToBox`
  (params (GameInfo :type "/Game/_Main/Blueprints/Structures/S_Game Structure"))
  (set `self.GameInfo` GameInfo)
  (`KismetSystemLibrary.Delay` 0.05)
  (for _index (range 1 (+ (`.UnitsPerBox_19_0C2495B344229AAEA74A76834BDC6F64` (break `/Game/_Main/Blueprints/Structures/S_Game` GameInfo)) 1))
    (bind _returnvalue (`|SpawnActorFromClass` "/Game/_Main/Blueprints/GameCase/BP_GameCase.BP_GameCase_C" (`SceneComponent.GetRelativeTransform` (`|GetArrayItem` (`self.GameCasesPlaces`) (- _index 1))) "Undefined" "MultiplyWithRoot" null null))
    (`/Game/_Main/Blueprints/GameCase/BP_GameCase.SetGameCase` _returnvalue (`self.GameInfo`))
    (`KismetArrayLibrary.Array_Add` (`self.GameCases`) _returnvalue)
    (`self.K2_AttachToComponent` _returnvalue (`self.SM_Equippable`) "None" "KeepRelative" "KeepRelative" "KeepRelative" true)))

(event `/Game/_Main/Blueprints/Interfaces/BPI_Interact.Interact`
  (params (CharacterRef :type "/Game/_Main/Blueprints/Character/BP_FirstPersonCharacter Object Reference"))
  (bind _sm_equippable (`self.SM_Equippable`))
  (`/Game/_Main/Blueprints/Character/BP_FirstPersonCharacter.Drop` CharacterRef)
  (`PrimitiveComponent.SetSimulatePhysics` _sm_equippable false)
  (`PrimitiveComponent.SetCollisionEnabled` _sm_equippable "NoCollision")
  (`self.K2_AttachToComponent` (`/Game/_Main/Blueprints/Character/BP_FirstPersonCharacter.BoxPoint` CharacterRef) "None" "SnapToTarget" "SnapToTarget" "SnapToTarget")
  (set `/Game/_Main/Blueprints/Character/BP_FirstPersonCharacter.EquippedActor` self CharacterRef))

(event `ClearBox`
  (`KismetArrayLibrary.Array_Clear` (`self.GameCases`))
  (set `self.Empty?` true))

(fn `UserConstructionScript`)