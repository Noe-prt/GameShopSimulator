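; BP_GameCase is a game case prop that displays a game's cover and can carry a price tag.
; SetGameCase stores the GameInfo and applies its material to the second material slot of the case mesh.
; PutPriceTag stores the price, writes it into the W_PriceTag widget and reveals the widget component, which starts hidden on BeginPlay.
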(event `self.ReceiveBeginPlay`
  (`SceneComponent.SetVisibility` (`self.PriceWidget`) false false))

(event `PutPriceTag`
  (params (Price :type "Float (double-precision)"))
  (set `self.Price` Price)
  (bind _asw_price_tag (cast `/Game/_Main/Widgets/W_PriceTag` (`WidgetComponent.GetUserWidgetObject` (`self.PriceWidget`))))
  (`/Game/_Main/Widgets/W_PriceTag.SetPriceText` _asw_price_tag Price)
  (`SceneComponent.SetVisibility` (`self.PriceWidget`) true false))

(event `SetGameCase`
  (params (GameInfo :type "/Game/_Main/Blueprints/Structures/S_Game Structure"))
  (set `self.GameInfo` GameInfo)
  (`PrimitiveComponent.SetMaterial` (`self.SM_GameCase`) 1 (`.Material_20_790C95624DA2D73FFBB902945FADF61A` (break `/Game/_Main/Blueprints/Structures/S_Game` GameInfo))))

(fn `UserConstructionScript`)