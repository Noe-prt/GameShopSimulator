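; BP_Slot is a slot that takes game cases from a delivery box and holds them with a shared price.
; Interact snaps the equipped box's cases onto ten preset places, applying the game mode's known price, or opens price input if already stocked.
; SetSlotPrice retags every case and restores game input and walking.
; Hover toggles a preview material and prompt; UpdateSlot removes the first case, resetting the slot when empty.
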(event `self.ReceiveBeginPlay`
  (set `self.GameCasesPlaces` (`|MakeArray` (`self.Box`) (`self.Box1`) (`self.Box2`) (`self.Box3`) (`self.Box4`) (`self.Box5`) (`self.Box6`) (`self.Box7`) (`self.Box8`) (`self.Box9`)))
  (set `self.SlotId` (`KismetSystemLibrary.GetDisplayName` self)))

(event `/Game/_Main/Blueprints/Interfaces/BPI_Hover.Hover/Unhover`
  (params (`Hover?` :type Boolean) (CharacterRef :type "/Game/_Main/Blueprints/Character/BP_FirstPersonCharacter Object Reference"))
  (bind _mainwidgetref (`/Game/_Main/Blueprints/Character/BP_FirstPersonCharacter.MainWidgetRef` CharacterRef))
  (if (`self.ContainGames`)
    (if `Hover?`
      (`PrimitiveComponent.SetMaterial` (`self.Cube`) 0 "/Game/_Main/Assets/Materials/MAT_Preview.MAT_Preview")
      (`/Game/_Main/Widgets/W_MainWidget.SpawnInteractBox` _mainwidgetref)
      (else
        (`PrimitiveComponent.SetMaterial` (`self.Cube`) 0 "/Game/_Main/Assets/Materials/M_Invisible.M_Invisible")
        (`/Game/_Main/Widgets/W_MainWidget.DespawnInteractBox` _mainwidgetref)))
    (else
      (bind _equippedactor (`/Game/_Main/Blueprints/Character/BP_FirstPersonCharacter.EquippedActor` CharacterRef)
        (:`then`
          (bind _asbp_delivery_box (cast `/Game/_Main/Blueprints/Delivery/BP_DeliveryBox` _equippedactor))
          (if (`/Game/_Main/Blueprints/Delivery/BP_DeliveryBox.Empty?` _asbp_delivery_box)
            _
            (elif `Hover?`
              (`PrimitiveComponent.SetMaterial` (`self.Cube`) 0 "/Game/_Main/Assets/Materials/MAT_Preview.MAT_Preview")
              (`/Game/_Main/Widgets/W_MainWidget.SpawnInteractBox` _mainwidgetref)
              (else
                (`PrimitiveComponent.SetMaterial` (`self.Cube`) 0 "/Game/_Main/Assets/Materials/M_Invisible.M_Invisible")
                (`/Game/_Main/Widgets/W_MainWidget.DespawnInteractBox` _mainwidgetref)))))
        (:`else`)))))

(event `/Game/_Main/Blueprints/Interfaces/BPI_Interact.Interact`
  (params (CharacterRef :type "/Game/_Main/Blueprints/Character/BP_FirstPersonCharacter Object Reference"))
  (set `self.Character Ref` CharacterRef)
  (if (`self.ContainGames`)
    (`/Game/_Main/Blueprints/Character/BP_FirstPersonCharacter.ShowPriceInputWidget` CharacterRef (`self.GameInfo`) (`self.Price`))
    (else
      (bind _equippedactor (`/Game/_Main/Blueprints/Character/BP_FirstPersonCharacter.EquippedActor` CharacterRef)
        (:`then`
          (bind _asbp_delivery_box (cast `/Game/_Main/Blueprints/Delivery/BP_DeliveryBox` _equippedactor))
          (if (not (`/Game/_Main/Blueprints/Delivery/BP_DeliveryBox.Empty?` _asbp_delivery_box))
            (bind _gamecases (`/Game/_Main/Blueprints/Delivery/BP_DeliveryBox.GameCases` _asbp_delivery_box))
            (set `self.GameCases` _gamecases)
            (bind _gamemoderef (message `/Game/_Main/Blueprints/Interfaces/BPI_GameMode.GetGameModeRef` (`GameplayStatics.GetGameMode`)))
            (bind _gameinfo (`/Game/_Main/Blueprints/Delivery/BP_DeliveryBox.GameInfo` _asbp_delivery_box))
            (bind (_found_ _price) (`/Game/_Main/Blueprints/GM_GameShopSimulator.GetGameCurrentPrice` _gamemoderef _gameinfo))
            (set `self.GameInfo` _gameinfo)
            (for (_array_element _array_index) _gamecases
              (`self.K2_DetachFromActor` _array_element "KeepRelative" "KeepRelative" "KeepRelative")
              (`self.K2_AttachToComponent` _array_element (`|GetArrayItem` (`self.GameCasesPlaces`) _array_index) "None" "SnapToTarget" "SnapToTarget" "SnapToTarget" true)
              (if _found_
                (`/Game/_Main/Blueprints/GameCase/BP_GameCase.PutPriceTag` _array_element _price)))
            (set `self.ContainGames` true)
            (`/Game/_Main/Blueprints/Delivery/BP_DeliveryBox.ClearBox` _asbp_delivery_box)
            (`PrimitiveComponent.SetMaterial` (`self.Cube`) 0 "/Game/_Main/Assets/Materials/M_Invisible.M_Invisible")
            (if _found_
              (set `self.Price` _price))))
        (:`else`)))))

(event `SetSlotPrice`
  (params (Price :type "Float (double-precision)"))
  (bind _returnvalue (`GameplayStatics.GetPlayerController` 0))
  (bind _output_get (set `self.Price` Price))
  (for _array_element (`self.GameCases`)
    (`/Game/_Main/Blueprints/GameCase/BP_GameCase.PutPriceTag` _array_element _output_get)
    (set `PlayerController.bShowMouseCursor` false _returnvalue)
    (`WidgetBlueprintLibrary.SetInputMode_GameOnly` _returnvalue)
    (`CharacterMovementComponent.SetMovementMode` (`Character.CharacterMovement` (`self.Character Ref`)) "MOVE_Walking" 0)))

(event `UpdateSlot`
  (`KismetArrayLibrary.Array_Remove` (`self.GameCases`))
  (if (`KismetArrayLibrary.Array_IsEmpty` (`self.GameCases`))
    (set `self.ContainGames` false)
    (set `self.Price` 0.0)
    (set `self.GameInfo` (struct))))

(fn `UserConstructionScript`)